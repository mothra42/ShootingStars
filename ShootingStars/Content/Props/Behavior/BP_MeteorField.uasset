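; BP_MeteorField is a meteor field prop Blueprint that holds a set of meteor spawn points.
; On BeginPlay it gathers sixteen individually named MeteorSpawn references into the SpawnPoints array, a hard-coded setup the author notes as provisional.
; The construction script is empty, and the graphs shown contain no logic that spawns meteors or reads the array.
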(event EventBeginPlay
  ;[1 1 1] Setup array of Spawn points, should be done more elegantly later.
  (Variables|Default|SetSpawnPoints (Utilities|Array|MakeArray (Variables|Default|GetMeteorSpawn8) (Variables|Default|GetMeteorSpawn1) (Variables|Default|GetMeteorSpawn2) (Variables|Default|GetMeteorSpawn3) (Variables|Default|GetMeteorSpawn4) (Variables|Default|GetMeteorSpawn5) (Variables|Default|GetMeteorSpawn6) (Variables|Default|GetMeteorSpawn7) (Variables|Default|GetMeteorSpawn) (Variables|Default|GetMeteorSpawn9) (Variables|Default|GetMeteorSpawn10) (Variables|Default|GetMeteorSpawn11) (Variables|Default|GetMeteorSpawn12) (Variables|Default|GetMeteorSpawn13) (Variables|Default|GetMeteorSpawn14) (Variables|Default|GetMeteorSpawn15))))

(fn ConstructionScript)