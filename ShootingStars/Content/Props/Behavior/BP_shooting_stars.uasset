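; Shooting star prop that moves itself between two marker actors placed in the level.
; On BeginPlay it finds the first actors tagged "start" and "end", and plays the Fall timeline only if both are valid.
; Each timeline update lerps its location between the two markers' current positions using the Fall track, without sweeping.
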(event EventBeginPlay
  (bind _outactors (Actor|GetAllActorswithTag "start"))
  (bind _outactors_2 (Actor|GetAllActorswithTag "end"))
  (Utilities|IsValid (Utilities|Array|Get(acopy) _outactors)
    (:Is%20Valid
      (Utilities|IsValid (Utilities|Array|Get(acopy) _outactors_2)
        (:Is%20Valid
          (bind _fall (Timeline|Fall Play)
            (:Update
              (Transformation|SetActorLocation (Math|Vector|Lerp(Vector) (Transformation|GetActorLocation (Utilities|Array|Get(acopy) _outactors)) (Transformation|GetActorLocation (Utilities|Array|Get(acopy) _outactors_2)) _fall) false false))))))))

(fn ConstructionScript)